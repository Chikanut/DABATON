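; DialogueSystem plays a dialogue line by ID as 2D voice-over with an optional timed subtitle.
; On BeginPlay it caches Settings and Localization from the ComposotionRoot game instance and creates the DialogueWidget in the viewport.
; PlayDialogue refetches Localization if missing, plays its VO, and sends its text to the widget when Subtitles is enabled.
; Failures print to screen, and disabled subtitles also print the "Settings info is NULL!" message.
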(event EventBeginPlay
  (CallFunction|UpdateInfo))

(fn ConstructionScript)

(fn PlayDialogue
  (params (ID :type String) (ShowTime :type Float%20%28single-precision%29))
  (bind _localization (Variables|Default|GetLocalization))
  (if (!= _localization 0)
    _
    (else
      (CallFunction|UpdateLocalization)))
  (CallFunction|PlayDialogueSound _localization ID)
  (CallFunction|PlayDialogueSubtitle ID ShowTime _localization))

(fn UpdateInfo
  (bind _ascomposotion_root (Utilities|Casting|CastToComposotionRoot (Game|GetGameInstance))
    (:then
      (bind _progress (Default|GetProgress _ascomposotion_root))
      (Variables|Default|SetSettings (Variables|/Game/BluePrints/Progress/ProgressManager.ProgressManager_C|GetSettings _progress))
      (CallFunction|UpdateUI)
      (CallFunction|UpdateLocalization))
    (:CastFailed
      (Development|PrintString "Game Instance is NULL!" true true "(R=0.713542,G=0.000000,B=0.000000,A=1.000000)"))))

(fn UpdateUI
  (if (== (Variables|Default|GetUI) 0)
    (bind _returnvalue (UserInterface|CreateWidget "/Game/BluePrints/DialogueSystem/DialogueWidget.DialogueWidget_C"))
    (bind _output_get (Variables|Default|SetUI _returnvalue))
    (UserInterface|Viewport|AddtoViewport _output_get 0)))

(fn UpdateLocalization
  (bind _ascomposotion_root (Utilities|Casting|CastToComposotionRoot (Game|GetGameInstance))
    (:then
      (bind _localization (Default|GetLocalization _ascomposotion_root))
      (Variables|Default|SetLocalization _localization))
    (:CastFailed
      (Development|PrintString "Game Instance is NULL!" true true "(R=0.713542,G=0.000000,B=0.000000,A=1.000000)"))))

(fn PlayDialogueSound
  (params (Localization :type Localization%20Manager%20Object%20Reference) (ID :type String))
  (bind _translation (Default|GetVO Localization ID))
  (if (!= _translation 0)
    (Audio|PlaySound2D _translation 1.0 1.0 0.0 0 0)
    (else
      (Development|PrintString (Utilities|String|Append "" " Dialogue sound is NULL") true true "(R=0.458333,G=0.012869,B=0.000000,A=1.000000)"))))

(fn PlayDialogueSubtitle
  (params (ID :type String) (Time :type Float%20%28single-precision%29) (Localization :type Localization%20Manager%20Object%20Reference))
  (bind _ui (Variables|Default|GetUI))
  (bind _settings (Variables|Default|GetSettings))
  (if (and (!= _settings 0) (Variables|/Game/BluePrints/Progress/Settings.Settings_C|GetSubtitles _settings))
    (bind _translation (Default|GetText Localization ID))
    (if (!= _ui 0)
      (Default|ShowDialogue _ui _translation Time)
      (else
        (Development|PrintString "Dialogue UI is NULL!" true true "(R=1.000000,G=0.008451,B=0.000000,A=1.000000)")))
    (else
      (Development|PrintString "Settings info is NULL!" true true "(R=1.000000,G=0.025572,B=0.000000,A=1.000000)"))))