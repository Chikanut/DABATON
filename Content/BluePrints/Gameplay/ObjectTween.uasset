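; Actor that ping-pongs itself between two points, such as for a simple moving object.
; At BeginPlay it turns StartPos and EndPos offsets into world positions relative to its root's location.
; Each Tick it advances Progress by DeltaSeconds over Time, lerps the root between the points, and flips Direction at either end.
; Progress is not clamped and is printed to screen every frame.
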(event EventTick
  (params (DeltaSeconds :type Float%20%28single-precision%29))
  (bind _output_get (Variables|Default|SetProgress (+ (* (Variables|Default|GetDirection) (/ DeltaSeconds (Variables|Default|GetTime))) (Variables|Default|GetProgress))))
  (Development|PrintString (Utilities|String|ToString(Float) _output_get))
  (Transformation|SetWorldLocation (Variables|Default|GetDefaultSceneRoot) (Math|Vector|Lerp(Vector) (Variables|Default|GetStartPos) (Variables|Default|GetEndPos) _output_get) false false)
  (Utilities|FlowControl|Sequence
    (:then_0
      (Math|Float|CompareFloat (Variables|Default|GetProgress) 1.0
        (:>
          _)
        (:==
          _))
      (Variables|Default|SetDirection -1.0))
    (:then_1
      (Math|Float|CompareFloat (Variables|Default|GetProgress) 0.0
        (:==
          _)
        (:<
          _))
      (Variables|Default|SetDirection 1.0))))

(event EventBeginPlay
  (Variables|Default|SetStartPos (+ (Variables|Default|GetStartPos) (Transformation|GetWorldLocation (Variables|Default|GetDefaultSceneRoot))))
  (Variables|Default|SetEndPos (+ (Variables|Default|GetEndPos) (Transformation|GetWorldLocation (Variables|Default|GetDefaultSceneRoot))))
  (Variables|Default|SetDirection 1.0))

(fn ConstructionScript)