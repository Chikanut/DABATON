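; DABATON game mode that bootstraps gameplay around the player's Hero pawn.
; On BeginPlay it casts player pawn 0 to Hero, stopping if that fails, and passes it to Init.
; Init stores the Hero, spawns an OasisManager at the game mode's root transform and initializes it with that Hero.
; CallOnInited then runs once setup completes.
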(event EventBeginPlay
  (bind _ashero (Utilities|Casting|CastToHero (Game|Player|GetPlayerPawn 0)))
  (CallFunction|Init _ashero)
  (Default|CallOnInited))

(fn ConstructionScript)

(fn Init
  (params (Hero :type Hero%20Object%20Reference))
  (bind _output_get (Variables|Default|SetHero Hero))
  (bind _returnvalue (Game|SpawnActorfromClass "/Game/BluePrints/Gameplay/Environment/OasisManager.OasisManager_C" (Transformation|GetWorldTransform (Variables|Default|GetDefaultSceneRoot)) "AlwaysSpawn" 0 0))
  (bind _output_get_2 (Variables|Default|SetOasisManager _returnvalue))
  (Default|Init _output_get_2 _output_get))