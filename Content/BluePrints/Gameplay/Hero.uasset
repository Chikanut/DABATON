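; Hero is the player character, with axis-driven movement, mouse look and jumping.
; Movement input follows the forward and right vectors of the control rotation.
; The Action input runs a Visibility line trace from the camera out to InteractionRadius, with debug drawing, and calls Use on a hit actor that casts to ButtonInterface.
; On BeginPlay it adds the UI widget to the viewport and hides the mouse cursor.
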(event EventBeginPlay
  (bind _returnvalue (UserInterface|CreateWidget "/Game/UI/UI.UI_C"))
  (UserInterface|Viewport|AddtoViewport _returnvalue 0)
  (Variables|/Script/Engine.PlayerController|SetbShowMouseCursor (Game|GetPlayerController 0) false))

(event Input|ActionEvents|InputActionJump
  (params (Key :type Key%20Structure :default "None"))
  ;[1 1 1] Physics Actions
  (:Pressed
    (Character|Jump)))

(event Input|ActionEvents|InputActionAction
  (params (Key :type Key%20Structure :default "None"))
  (bind _camera (Variables|Default|GetCamera))
  (bind _returnvalue (Transformation|GetWorldLocation _camera))
  ;[1 1 1] Interaction
  (:Pressed
    (bind (_outhit _returnvalue_2) (Collision|LineTraceByChannel _returnvalue (+ _returnvalue (* (Math|Vector|GetForwardVector _camera) (Variables|Default|GetInteraction%20Radius))) "TraceTypeQuery1" false 0 "ForDuration"))
    (if _returnvalue_2
      (bind _asbutton_interface (Utilities|Casting|CastToButtonInterface (.HitActor (Collision|BreakHitResult _outhit))))
      (Default|Use _asbutton_interface))))

(event Input|AxisEvents|InputAxisVertical
  (params (AxisValue :type Float%20%28single-precision%29))
  ;[1 1 1] Vertical Movement
  (Pawn|Input|AddMovementInput (Math|Vector|GetForwardVector (Pawn|GetControlRotation :!class /Script/Engine.Pawn)) AxisValue false))

(event Input|AxisEvents|InputAxisHorizontal
  (params (AxisValue :type Float%20%28single-precision%29))
  ;[1 1 1] Horizontal Movement
  (Pawn|Input|AddMovementInput (Math|Vector|GetRightVector (Pawn|GetControlRotation :!class /Script/Engine.Pawn)) AxisValue false))

(event Input|AxisEvents|InputAxisLook_Horizontal
  (params (AxisValue :type Float%20%28single-precision%29))
  ;[1 1 1] Mouse
  (Pawn|Input|AddControllerYawInput AxisValue))

(event Input|AxisEvents|InputAxisLook_Vertical
  (params (AxisValue :type Float%20%28single-precision%29))
  ;[1 1 1] Mouse
  (Pawn|Input|AddControllerPitchInput AxisValue))

(fn ConstructionScript)