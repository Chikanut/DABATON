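; Wire actor that draws a simulated rope as spline meshes and, when used, sets the user as the rope's target.
; Each tick it rebuilds the spline from the Rope particle positions, setting interior tangents toward the next point with a capped length.
; It then fits spline mesh components to the segments, reusing a pool that grows on demand and hides surplus meshes.
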(event EventBeginPlay
  (Default|Init (Variables|Default|GetRope) self))

(event EventTick
  (params (DeltaSeconds :type Float%20%28single-precision%29))
  (CallFunction|UpdateSpline)
  (CallFunction|UpdateMesh))

(event EventUse
  (params (User :type Hero%20Object%20Reference))
  (Default|SetTarget (Variables|Default|GetRope) User))

(fn ConstructionScript)

(fn UpdateSpline
  (bind _spline (Variables|Default|GetSpline))
  (bind _rope (Variables|Default|GetRope))
  (bind _spline_2 (Variables|Default|GetSpline))
  (bind _particles (Variables|/Game/BluePrints/Gameplay/RopeComponent.RopeComponent_C|GetParticles _rope))
  (bind _returnvalue (Utilities|Array|Length _particles))
  (Spline|ClearSplinePoints (Variables|Default|GetSpline) false)
  (for (_array_element _array_index) (Variables|/Game/BluePrints/Gameplay/RopeComponent.RopeComponent_C|GetParticles (Variables|Default|GetRope))
    (LocalVariables|SetCurrentIndex _array_index)
    (Spline|AddSplinePoint _spline_2 (.Position (Utilities|Struct|BreakRopeParticle _array_element)) "World" false)
    (Spline|SetSplinePointType _spline_2 (LocalVariables|GetCurrentIndex) "Curve" true))
  (for _index (range 0 (Spline|GetNumberOfSplinePoints (Variables|Default|GetSpline)))
    (bind _output_get (LocalVariables|SetCurrentIndex _index))
    (Math|Integer|CompareInt _output_get
      (:>
        (Math|Integer|CompareInt _returnvalue 2
          (:>
            (Math|Integer|CompareInt (LocalVariables|GetCurrentIndex) (- _returnvalue 1)
              (:<
                (Spline|SetTangentatSplinePoint _spline (LocalVariables|GetCurrentIndex) (* (Math|Vector|GetUnitDirection(Vector) (Spline|GetLocationatSplinePoint _spline (LocalVariables|GetCurrentIndex) "World") (Spline|GetLocationatSplinePoint _spline (+ (LocalVariables|GetCurrentIndex) 1) "World")) (Math|Float|Clamp(Float) (/ (Math|Vector|Distance(Vector) (Spline|GetLocationatSplinePoint _spline (+ (LocalVariables|GetCurrentIndex) 1) "World") (Spline|GetLocationatSplinePoint _spline (LocalVariables|GetCurrentIndex) "World")) 2.0) -25.0 25.0)) "World" true)))))))))

(fn UpdateMesh
  (bind _spline (Variables|Default|GetSpline))
  (bind _spline_2 (Variables|Default|GetSpline))
  (bind _meshes (Variables|Default|GetMeshes))
  (bind _returnvalue (Utilities|Array|Length _meshes))
  (bind _returnvalue_2 (Spline|GetNumberOfSplinePoints _spline))
  (bind _returnvalue_3 (- _returnvalue_2 2))
  (bind _returnvalue_4 (Math|Integer|Clamp(Integer) _returnvalue_3 0 _returnvalue_2))
  (Math|Integer|CompareInt _returnvalue _returnvalue_4
    (:>
      (for _index (range _returnvalue_4 (Math|Integer|Clamp(Integer) (- _returnvalue 1) 0 _returnvalue))
        (Rendering|SetVisibility (Utilities|Array|Get(acopy) (Variables|Default|GetMeshes) _index) false false)))
    (:==
      _)
    (:<
      _))
  (for _index_2 (range 0 (- (Spline|GetNumberOfSplinePoints _spline) 2))
    (Math|Integer|CompareInt _index_2 (Utilities|Array|Length (Variables|Default|GetMeshes))
      (:>
        (bind _returnvalue_5 (AddComponent|AddSplineMeshComponent false :!label _label))
        (Utilities|Array|Add (Variables|Default|GetMeshes) _returnvalue_5))
      (:==
        (goto _label))
      (:<
        _))
    (SplineMesh|SetStartandEnd (Utilities|Array|Get(acopy) (Variables|Default|GetMeshes) _index_2) (Spline|GetLocationatSplinePoint _spline_2 _index_2 "Local") (Spline|GetTangentatSplinePoint _spline_2 _index_2 "Local") (Spline|GetLocationatSplinePoint _spline_2 (+ _index_2 1) "Local") (Spline|GetTangentatSplinePoint _spline_2 (+ _index_2 1) "Local") true :!class /Script/Engine.SplineMeshComponent)
    (Rendering|SetVisibility (Utilities|Array|Get(acopy) (Variables|Default|GetMeshes) _index_2) true false)))