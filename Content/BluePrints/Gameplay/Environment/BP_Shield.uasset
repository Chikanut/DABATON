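; BP_Shield is an environment actor that stamps its location into the OasisTexture render target using a brush material.
; The construction script creates a dynamic instance of OasisBrush as BrushMID.
; DrawAtLocation passes the actor's position, Size and Strength to that instance, then draws it to the render target; nothing in this Blueprint calls the event.
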(event Custom|DrawAtLocation
  (Rendering|Material|SetVectorParameterValue (Variables|Default|GetBrushMID) "Position" (Math|Conversions|ToLinearColor(Vector) (Transformation|GetActorLocation)) :!class /Script/Engine.MaterialInstanceDynamic)
  (Rendering|Material|SetScalarParameterValue (Variables|Default|GetBrushMID) "Size" (Variables|Default|GetSize) :!class /Script/Engine.MaterialInstanceDynamic)
  (Rendering|Material|SetScalarParameterValue (Variables|Default|GetBrushMID) "Strength" (Variables|Default|GetStrength) :!class /Script/Engine.MaterialInstanceDynamic)
  (Rendering|DrawMaterialtoRenderTarget "/Game/Textures/OasisTexture.OasisTexture" (Variables|Default|GetBrushMID)))

(fn ConstructionScript
  (bind _returnvalue (Rendering|Material|CreateDynamicMaterialInstance "/Game/Materials/Brush/OasisBrush.OasisBrush" "None" :!class /Script/Engine.KismetMaterialLibrary))
  (Variables|Default|SetBrushMID _returnvalue))