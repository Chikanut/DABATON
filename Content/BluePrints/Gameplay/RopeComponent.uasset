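; Rope component that stretches between its actor and a target set via SetTarget, wrapping around geometry.
; Each tick pipes the particle array through anchor updates, bend-point insertion at sphere-trace hits (count-capped), surface re-snapping, friction and pruning.
; Friction slides bend points toward the line between their neighbours by angle, while pruning removes or re-projects points by contact and angle.
; The rope renders only as debug lines and spheres.
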(event Custom|SetTarget
  (params (NewTarget :type Actor%20Object%20Reference))
  (Variables|Default|SetTarget NewTarget)
  (Variables|Default|SetActive true)
  (bind _particles (CallFunction|CombineParticles))
  (Variables|Default|SetParticles _particles))

(event Custom|Init
  (params (this :type Actor%20Object%20Reference))
  (Variables|Default|SetThis this))

(event EventTick
  (params (DeltaSeconds :type Float%20%28single-precision%29))
  (if (Variables|Default|GetActive)
    (bind _outparticles (CallFunction|UpdateAnchors (Variables|Default|GetParticles)))
    (bind _outparticles_2 (CallFunction|CheckforCollisions _outparticles))
    (bind _outparticles_3 (CallFunction|UpdateColliders _outparticles_2))
    (bind _outparticles_4 (CallFunction|UpdateFriction _outparticles_3 DeltaSeconds))
    (bind _outparticless (CallFunction|ClearFreeParticles _outparticles_4))
    (bind _output_get (Variables|Default|SetParticles _outparticless))
    (CallFunction|Visualise _output_get)))

(fn CombineParticles
  (bind _new_particles (LocalVariables|GetNew%20Particles))
  (Utilities|Array|Add _new_particles (Utilities|Struct|MakeRopeParticle (Transformation|GetActorLocation (Variables|Default|GetThis)) "0.000000,0.000000,0.000000"))
  (Utilities|Array|AppendArray _new_particles (Variables|Default|GetParticles))
  (Utilities|Array|Add _new_particles (Utilities|Struct|MakeRopeParticle (Transformation|GetActorLocation (Variables|Default|GetTarget)) "0.000000,0.000000,0.000000"))
  (return (LocalVariables|GetNew%20Particles)))

(fn ClearFreeParticles
  (params (InParticless :type Array%20of%20Rope%20Particle%20Structures))
  (bind _output_get (LocalVariables|SetReturnArray InParticless))
  (for (_ _array_index) _output_get
    (bind _output_get_2 (LocalVariables|SetCurrentIndex _array_index))
    (Math|Integer|CompareInt _output_get_2 0
      (:>
        (Math|Integer|CompareInt _output_get_2 (- (Utilities|Array|Length (LocalVariables|GetReturnArray)) 1)
          (:<
            (Math|Integer|CompareInt (Utilities|Array|Length (LocalVariables|GetReturnArray)) 2
              (:>
                (bind _returnvalue (Collision|SphereTraceForObjects (.Position (Utilities|Struct|BreakRopeParticle (Utilities|Array|Get(acopy) (LocalVariables|GetReturnArray) (LocalVariables|GetCurrentIndex)))) (+ (.Position (Utilities|Struct|BreakRopeParticle (Utilities|Array|Get(acopy) (LocalVariables|GetReturnArray) (LocalVariables|GetCurrentIndex)))) (* (.Normal (Utilities|Struct|BreakRopeParticle (Utilities|Array|Get(acopy) (LocalVariables|GetReturnArray) (LocalVariables|GetCurrentIndex)))) (* (Variables|Default|GetWidth) -2.0))) (* (Variables|Default|GetWidth) 1.1) (Variables|Default|GetTargetObjects) false (Utilities|Array|MakeArray (Variables|Default|GetTarget)) "None"))
                (if _returnvalue
                  (Math|Float|CompareFloat (Class|KismetMathLibrary|DegAcos (Math|Vector|DotProduct (Math|Vector|GetUnitDirection(Vector) (.Position (Utilities|Struct|BreakRopeParticle (Utilities|Array|Get(acopy) (LocalVariables|GetReturnArray) (LocalVariables|GetCurrentIndex)))) (Math|Vector|FindClosestPointonSegment (.Position (Utilities|Struct|BreakRopeParticle (Utilities|Array|Get(acopy) (LocalVariables|GetReturnArray) (LocalVariables|GetCurrentIndex)))) (.Position (Utilities|Struct|BreakRopeParticle (Utilities|Array|Get(acopy) (LocalVariables|GetReturnArray) (+ (LocalVariables|GetCurrentIndex) 1)))) (.Position (Utilities|Struct|BreakRopeParticle (Utilities|Array|Get(acopy) (LocalVariables|GetReturnArray) (- (LocalVariables|GetCurrentIndex) 1)))))) (Math|Vector|GetUnitDirection(Vector) (.Position (Utilities|Struct|BreakRopeParticle (Utilities|Array|Get(acopy) (LocalVariables|GetReturnArray) (LocalVariables|GetCurrentIndex)))) (.Position (Utilities|Struct|BreakRopeParticle (Utilities|Array|Get(acopy) (LocalVariables|GetReturnArray) (+ (LocalVariables|GetCurrentIndex) 1))))))) 1.1e+02
                    (:>
                      (bind (_outhit _returnvalue_2) (Collision|SphereTraceForObjects (.Position (Utilities|Struct|BreakRopeParticle (Utilities|Array|Get(acopy) (LocalVariables|GetReturnArray) (+ (LocalVariables|GetCurrentIndex) 1)))) (.Position (Utilities|Struct|BreakRopeParticle (Utilities|Array|Get(acopy) (LocalVariables|GetReturnArray) (- (LocalVariables|GetCurrentIndex) 1)))) (Variables|Default|GetWidth) (Variables|Default|GetTargetObjects) false (Utilities|Array|MakeArray (Variables|Default|GetTarget)) "None"))
                      (if _returnvalue_2
                        (bind (_outhit_2 _returnvalue_3) (Collision|SphereTraceForObjects (.Position (Utilities|Struct|BreakRopeParticle (Utilities|Array|Get(acopy) (LocalVariables|GetReturnArray) (LocalVariables|GetCurrentIndex)))) (.Location (Collision|BreakHitResult _outhit)) (Variables|Default|GetWidth) (Variables|Default|GetTargetObjects) false (Utilities|Array|MakeArray (Variables|Default|GetTarget)) "None"))
                        (if _returnvalue_3
                          (Utilities|Array|SetArrayElem (LocalVariables|GetReturnArray) (LocalVariables|GetCurrentIndex) (Utilities|Struct|MakeRopeParticle (+ (.Location (Collision|BreakHitResult _outhit_2)) (* (.Normal (Collision|BreakHitResult _outhit_2)) (/ (Variables|Default|GetWidth) 2.0))) (.Normal (Collision|BreakHitResult _outhit_2))))
                          (else
                            (Utilities|Array|RemoveIndex (LocalVariables|GetReturnArray) (LocalVariables|GetCurrentIndex) :!label _label)))
                        (else
                          (goto _label)))))
                  (else
                    (Utilities|Array|RemoveIndex (LocalVariables|GetReturnArray) (LocalVariables|GetCurrentIndex)))))))))))
  (return (LocalVariables|GetReturnArray)))

(fn CheckforCollisions
  (params (InputArray :type Array%20of%20Rope%20Particle%20Structures))
  (bind _output_get (LocalVariables|SetReturnArray InputArray))
  (for (_ _array_index) _output_get
    (bind _output_get_2 (LocalVariables|SetCurrentIndex _array_index))
    (Math|Integer|CompareInt _output_get_2
      (:>
        (bind (_outhit _returnvalue) (Collision|SphereTraceForObjects (.Position (Utilities|Struct|BreakRopeParticle (Utilities|Array|Get(acopy) (LocalVariables|GetReturnArray) (LocalVariables|GetCurrentIndex)))) (.Position (Utilities|Struct|BreakRopeParticle (Utilities|Array|Get(acopy) (LocalVariables|GetReturnArray) (- (LocalVariables|GetCurrentIndex) 1)))) (Variables|Default|GetWidth) (Variables|Default|GetTargetObjects) false (Utilities|Array|MakeArray (Variables|Default|GetTarget)) "None"))
        (if _returnvalue
          (Utilities|Array|Insert (LocalVariables|GetReturnArray) (Utilities|Struct|MakeRopeParticle (+ (.Location (Collision|BreakHitResult _outhit)) (* (.Normal (Collision|BreakHitResult _outhit)) (/ (Variables|Default|GetWidth) 2.0))) (.Normal (Collision|BreakHitResult _outhit))) (LocalVariables|GetCurrentIndex))
          (bind _result (Math|Integer|IncrementInt (LocalVariables|GetCurrentUpdates))
            (:%20%20
              (Math|Integer|CompareInt _result (Variables|Default|GetUpdates)
                (:>
                  _)
                (:==
                  _))
              (return (LocalVariables|GetReturnArray))))))))
  (return (LocalVariables|GetReturnArray)))

(fn UpdateFriction
  (params (InParticles :type Array%20of%20Rope%20Particle%20Structures) (DeltaTime :type Float%20%28single-precision%29))
  (bind _width (Variables|Default|GetWidth))
  (LocalVariables|SetDelta DeltaTime)
  (bind _output_get (LocalVariables|SetReturnArray InParticles))
  (for (_ _array_index) _output_get
    (bind _output_get_2 (LocalVariables|SetCurrentIndex _array_index))
    (Math|Integer|CompareInt _output_get_2
      (:>
        (Math|Integer|CompareInt _output_get_2 (- (Utilities|Array|Length (LocalVariables|GetReturnArray)) 1)
          (:<
            (Math|Integer|CompareInt (Utilities|Array|Length (LocalVariables|GetReturnArray)) 2
              (:>
                (bind _output_get_3 (LocalVariables|SetCurrentPos (.Position (Utilities|Struct|BreakRopeParticle (Utilities|Array|Get(acopy) (LocalVariables|GetReturnArray) (LocalVariables|GetCurrentIndex))))))
                (bind _output_get_4 (LocalVariables|SetCurrentNormal (.Normal (Utilities|Struct|BreakRopeParticle (Utilities|Array|Get(acopy) (LocalVariables|GetReturnArray) (LocalVariables|GetCurrentIndex))))))
                (LocalVariables|SetTargetPos (+ (* (Math|Vector|GetUnitDirection(Vector) (.Position (Utilities|Struct|BreakRopeParticle (Utilities|Array|Get(acopy) (LocalVariables|GetReturnArray) (LocalVariables|GetCurrentIndex)))) (Math|Vector|FindClosestPointonSegment (.Position (Utilities|Struct|BreakRopeParticle (Utilities|Array|Get(acopy) (LocalVariables|GetReturnArray) (LocalVariables|GetCurrentIndex)))) (.Position (Utilities|Struct|BreakRopeParticle (Utilities|Array|Get(acopy) (LocalVariables|GetReturnArray) (- (LocalVariables|GetCurrentIndex) 1)))) (.Position (Utilities|Struct|BreakRopeParticle (Utilities|Array|Get(acopy) (LocalVariables|GetReturnArray) (+ (LocalVariables|GetCurrentIndex) 1)))))) (* (Variables|Default|GetWidth) 2.0)) (.Position (Utilities|Struct|BreakRopeParticle (Utilities|Array|Get(acopy) (LocalVariables|GetReturnArray) (LocalVariables|GetCurrentIndex))))))
                (bind _returnvalue (Collision|SphereTraceForObjects _output_get_3 (+ (* (* _output_get_4 -1.0) _width) _output_get_3) _width (Variables|Default|GetTargetObjects) false (Utilities|Array|MakeArray (Variables|Default|GetTarget)) "ForOneFrame"))
                (if _returnvalue
                  (Utilities|Array|SetArrayElem (LocalVariables|GetReturnArray) (LocalVariables|GetCurrentIndex) (Utilities|Struct|MakeRopeParticle (+ (LocalVariables|GetCurrentPos) (* (Math|Vector|GetUnitDirection(Vector) (LocalVariables|GetCurrentPos) (LocalVariables|GetTargetPos)) (/ (LocalVariables|GetDelta) (/ (Variables|Default|GetFriction) (* 1e+02 (Math|Float|Clamp(Float) (- 1.0 (/ (Class|KismetMathLibrary|DegAcos (Math|Vector|DotProduct (Math|Vector|GetUnitDirection(Vector) (.Position (Utilities|Struct|BreakRopeParticle (Utilities|Array|Get(acopy) (LocalVariables|GetReturnArray) (LocalVariables|GetCurrentIndex)))) (Math|Vector|FindClosestPointonSegment (.Position (Utilities|Struct|BreakRopeParticle (Utilities|Array|Get(acopy) (LocalVariables|GetReturnArray) (LocalVariables|GetCurrentIndex)))) (.Position (Utilities|Struct|BreakRopeParticle (Utilities|Array|Get(acopy) (LocalVariables|GetReturnArray) (- (LocalVariables|GetCurrentIndex) 1)))) (.Position (Utilities|Struct|BreakRopeParticle (Utilities|Array|Get(acopy) (LocalVariables|GetReturnArray) (+ (LocalVariables|GetCurrentIndex) 1)))))) (Math|Vector|GetUnitDirection(Vector) (.Position (Utilities|Struct|BreakRopeParticle (Utilities|Array|Get(acopy) (LocalVariables|GetReturnArray) (LocalVariables|GetCurrentIndex)))) (.Position (Utilities|Struct|BreakRopeParticle (Utilities|Array|Get(acopy) (LocalVariables|GetReturnArray) (+ (LocalVariables|GetCurrentIndex) 1))))))) 9e+01)))))))) (LocalVariables|GetCurrentNormal)))))))))))
  (return (LocalVariables|GetReturnArray)))

(fn Visualise
  (params (Info :type Array%20of%20Rope%20Particle%20Structures))
  (for (_array_element _array_index) Info
    (Math|Integer|CompareInt _array_index
      (:>
        (Rendering|Debug|DrawDebugLine :LineStart (.Position (Utilities|Struct|BreakRopeParticle _array_element)) :LineEnd (.Position (Utilities|Struct|BreakRopeParticle (Utilities|Array|Get(acopy) (Variables|Default|GetParticles) (- _array_index 1)))))
        (Rendering|Debug|DrawDebugSphere (.Position (Utilities|Struct|BreakRopeParticle (Utilities|Array|Get(acopy) (Variables|Default|GetParticles) (- _array_index 1)))) (Variables|Default|GetWidth) 12 "(R=1.000000,G=1.000000,B=1.000000,A=1.000000)" 0.0)))))

(fn UpdateColliders
  (params (InParticles :type Array%20of%20Rope%20Particle%20Structures))
  (bind _width (Variables|Default|GetWidth))
  (bind _output_get (LocalVariables|SetReturnArray InParticles))
  (for (_ _array_index) _output_get
    (LocalVariables|SetCurrentIndex _array_index)
    (bind (_outhit _returnvalue) (Collision|SphereTraceForObjects (+ (.Position (Utilities|Struct|BreakRopeParticle (Utilities|Array|Get(acopy) (LocalVariables|GetReturnArray) (LocalVariables|GetCurrentIndex)))) (* (.Normal (Utilities|Struct|BreakRopeParticle (Utilities|Array|Get(acopy) (LocalVariables|GetReturnArray) (LocalVariables|GetCurrentIndex)))) (* _width 2.0))) (+ (.Position (Utilities|Struct|BreakRopeParticle (Utilities|Array|Get(acopy) (LocalVariables|GetReturnArray) (LocalVariables|GetCurrentIndex)))) (* (.Normal (Utilities|Struct|BreakRopeParticle (Utilities|Array|Get(acopy) (LocalVariables|GetReturnArray) (LocalVariables|GetCurrentIndex)))) (* _width -2.0))) (Variables|Default|GetWidth) (Variables|Default|GetTargetObjects) false (Utilities|Array|MakeArray (Variables|Default|GetTarget)) "None"))
    (if _returnvalue
      (Utilities|Array|SetArrayElem (LocalVariables|GetReturnArray) (LocalVariables|GetCurrentIndex) (Utilities|Struct|MakeRopeParticle (+ (.Location (Collision|BreakHitResult _outhit)) (* (.Normal (Collision|BreakHitResult _outhit)) (/ (Variables|Default|GetWidth) 2.0))) (.Normal (Collision|BreakHitResult _outhit))))))
  (return (LocalVariables|GetReturnArray)))

(fn UpdateAnchors
  (params (InParticles :type Array%20of%20Rope%20Particle%20Structures))
  (Utilities|Array|SetArrayElem InParticles 0 (Utilities|Struct|MakeRopeParticle (Transformation|GetActorLocation (Variables|Default|GetThis)) "0.000000,0.000000,0.000000"))
  (bind _result (Math|Integer|DecrementInt (Utilities|Array|Length InParticles))
    (:%20%20
      (Utilities|Array|SetArrayElem InParticles _result (Utilities|Struct|MakeRopeParticle (Transformation|GetActorLocation (Variables|Default|GetTarget)) "0.000000,0.000000,0.000000"))
      (return InParticles))))