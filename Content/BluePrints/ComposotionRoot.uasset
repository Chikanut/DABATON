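; ComposotionRoot is a composition root that creates and hands out the game's Progress, Localization, Audio and Dialogue managers.
; Each getter lazily calls its init function when the cached reference is unset, which spawns the manager actor and stores it.
; Audio also runs its own Init after spawning, and only the Dialogue init guards itself against double creation.
; The Init event is empty.
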(event EventInit)

(fn GetProgress
  (if (!= (Variables|Default|GetProgress) 0)
    _
    (else
      (CallFunction|InitProgress)))
  (return (Variables|Default|GetProgress)))

(fn InitProgress
  (params (Parent :type Transform))
  (bind _returnvalue (Game|SpawnActorfromClass "/Game/BluePrints/Progress/ProgressManager.ProgressManager_C" Parent "Undefined" 0 0))
  (Variables|Default|SetProgress _returnvalue)
  (Development|PrintString "Progress manager Inited!"))

(fn InitLocalization
  (params (Parent :type Transform))
  (bind _returnvalue (Game|SpawnActorfromClass "/Game/BluePrints/Localization/LocalizationManager.LocalizationManager_C" Parent "Undefined" 0 0))
  (Variables|Default|SetLocalization _returnvalue))

(fn GetLocalization
  (if (!= (Variables|Default|GetLocalization) 0)
    _
    (else
      (CallFunction|InitLocalization)))
  (return (Variables|Default|GetLocalization)))

(fn InitAudio
  (params (Parent :type Transform))
  (bind _returnvalue (Game|SpawnActorfromClass "/Game/BluePrints/AudioManager/AudioManager.AudioManager_C" Parent "Undefined" 0 0))
  (bind _output_get (Variables|Default|SetAudio _returnvalue))
  (Default|Init _output_get))

(fn GetAudio
  (if (!= (Variables|Default|GetAudio) 0)
    _
    (else
      (CallFunction|InitAudio)))
  (return (Variables|Default|GetAudio)))

(fn InitDialogue
  (params (Parent :type Transform))
  (if (== (Variables|Default|GetDialogue) 0)
    (bind _returnvalue (Game|SpawnActorfromClass "/Game/BluePrints/DialogueSystem/DialogueSystem.DialogueSystem_C" Parent "Undefined" 0 0))
    (Variables|Default|SetDialogue _returnvalue)))

(fn GetDialogue
  (if (!= (Variables|Default|GetDialogue) 0)
    _
    (else
      (CallFunction|InitDialogue)))
  (return (Variables|Default|GetDialogue)))