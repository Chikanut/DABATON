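; AudioManager applies the player's saved volume settings to the game's DABATON sound mix.
; On BeginPlay it sets the base sound mix and runs Init, which UpdateSettings also calls to reapply changes.
; Init reads Settings from the ComposotionRoot game instance's progress and overrides the Sounds, Music and Master sound class volumes.
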(event Custom|UpdateSettings
  (CallFunction|Init))

(event EventBeginPlay
  (Class|GameplayStatics|SetBaseSoundMix "/Game/BluePrints/AudioManager/DABATON_SoundMix.DABATON_SoundMix")
  (CallFunction|Init))

(fn ConstructionScript)

(fn Init
  (bind _ascomposotion_root (Utilities|Casting|CastToComposotionRoot (Game|GetGameInstance)))
  (bind _progress (Default|GetProgress _ascomposotion_root))
  (Audio|SetSoundMixClassOverride "/Game/BluePrints/AudioManager/DABATON_SoundMix.DABATON_SoundMix" "/Game/BluePrints/AudioManager/DABATON_Sounds.DABATON_Sounds" (Variables|/Game/BluePrints/Progress/Settings.Settings_C|GetSounds%20Volume (Variables|/Game/BluePrints/Progress/ProgressManager.ProgressManager_C|GetSettings _progress)) 1.0 1.0 true)
  (Audio|SetSoundMixClassOverride "/Game/BluePrints/AudioManager/DABATON_SoundMix.DABATON_SoundMix" "/Game/BluePrints/AudioManager/DABATON_Music.DABATON_Music" (Variables|/Game/BluePrints/Progress/Settings.Settings_C|GetMusic%20Volume (Variables|/Game/BluePrints/Progress/ProgressManager.ProgressManager_C|GetSettings _progress)) 1.0 1.0 true)
  (Audio|SetSoundMixClassOverride "/Game/BluePrints/AudioManager/DABATON_SoundMix.DABATON_SoundMix" "/Game/BluePrints/AudioManager/DABATON_Master.DABATON_Master" (Variables|/Game/BluePrints/Progress/Settings.Settings_C|GetMaster%20Volume (Variables|/Game/BluePrints/Progress/ProgressManager.ProgressManager_C|GetSettings _progress)) 1.0 1.0 true))