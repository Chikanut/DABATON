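; PlayerProgress tracks the player's current level and resolves it against the Levels data table.
; Level names come from indexing the table's row names by level number, with a printed error and "None" when the row is missing.
; IsNextLevel compares CurrentLevel to the last index of the LevelName column to report whether another level follows.
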(fn GetLevelName
  (params (LevelNum :type Integer))
  (bind _levels (Variables|Default|GetLevels))
  (bind _outrownames (DataTable|GetDataTableRowNames _levels))
  (bind _returnvalue (Utilities|GetDataTableRow _levels (Utilities|Array|Get(acopy) _outrownames LevelNum))
    (:then
      (return (Utilities|Struct|BreakLevelsStructure _returnvalue)))
    (:RowNotFound
      (Development|PrintString 0 "Level not found!" true true "(R=1.000000,G=0.008232,B=0.000000,A=1.000000)")
      (return "None"))))

(fn GetCurrentLevelName
  (bind _levelname (CallFunction|GetLevelName (Variables|Default|GetCurrentLevel)))
  (return _levelname))

(fn IsNextLevel
  (bind _returnvalue (Class|DataTableFunctionLibrary|GetDataTableColumnasString (Variables|Default|GetLevels) "LevelName"))
  (Math|Integer|CompareInt (Variables|Default|GetCurrentLevel) (- (Utilities|Array|Length _returnvalue) 1)
    (:>
      _)
    (:==
      _)
    (:<
      (return true)))
  (return false))