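; ProgressManager is an actor that persists the game's settings and player progress through save games.
; On BeginPlay it loads the Settings and Progress slots into variables, creating a fresh save object whenever a load or cast fails.
; On EndPlay it writes both objects back to their slots, first creating a new one if either reference is missing.
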(event EventBeginPlay
  ;[1 1 1] Load Info On Start
  (bind _returnvalue (SaveGame|LoadGamefromSlot "Settings"))
  (bind _assettings (Utilities|Casting|CastToSettings _returnvalue)
    (:then
      (Variables|Default|SetSettings _assettings))
    (:CastFailed
      (bind _returnvalue_2 (SaveGame|CreateSaveGameObject "/Game/BluePrints/Progress/Settings.Settings_C"))
      (Variables|Default|SetSettings _returnvalue_2)))
  (bind _returnvalue_3 (SaveGame|LoadGamefromSlot "Progress"))
  (bind _asplayer_progress (Utilities|Casting|CastToPlayerProgress _returnvalue_3)
    (:then
      (Variables|Default|SetProgress _asplayer_progress))
    (:CastFailed
      (bind _returnvalue_4 (SaveGame|CreateSaveGameObject "/Game/BluePrints/Progress/PlayerProgress.PlayerProgress_C"))
      (Variables|Default|SetProgress _returnvalue_4))))

(event EventEndPlay
  (params (EndPlayReason :type EEndPlayReason%20Enum :default "Destroyed"))
  ;[1 1 1] Save Info On Finish
  (if (!= (Variables|Default|GetSettings) 0)
    _
    (else
      (bind _returnvalue (SaveGame|CreateSaveGameObject "/Game/BluePrints/Progress/Settings.Settings_C"))
      (Variables|Default|SetSettings _returnvalue)))
  (SaveGame|SaveGametoSlot (Variables|Default|GetSettings) "Settings")
  (if (!= (Variables|Default|GetProgress) 0)
    _
    (else
      (bind _returnvalue_2 (SaveGame|CreateSaveGameObject "/Game/BluePrints/Progress/PlayerProgress.PlayerProgress_C"))
      (Variables|Default|SetProgress _returnvalue_2)))
  (SaveGame|SaveGametoSlot (Variables|Default|GetProgress) "Progress"))

(fn ConstructionScript)